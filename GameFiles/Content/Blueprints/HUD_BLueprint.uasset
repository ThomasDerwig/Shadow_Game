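; HUD Blueprint that creates the player's on-screen widgets and handles background audio.
; On BeginPlay it adds the normal HUD, sets a custom widget cursor and starts the Audio component.
; Events show a two-second "more friends needed" gate text, a death screen on enemy interaction, or a win screen.
; CollectAll plays a sound cue and stops the audio before the win screen, while ExitLevel jumps straight to that screen.
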(event `/Game/Interactions/Gate_Interact.MoreFriendsNeeded`
  ;[1 1 1] gate text
  (bind _returnvalue (`|CreateWidget` "/Game/HUD_messages/Text.Text_C" (`GameplayStatics.GetPlayerController` 0)))
  (`UserWidget.AddToViewport` _returnvalue 0)
  (`KismetSystemLibrary.Delay` 2.0)
  (`KismetSystemLibrary.PrintString` "delaylo")
  (`Widget.RemoveFromParent` _returnvalue))

(event `self.ReceiveBeginPlay`
  (bind _returnvalue (`GameplayStatics.GetPlayerController` 0))
  ;[1 1 1] Setup
  (`|ExecutionSequence`
    (:`then_0`
      (bind _returnvalue_2 (`|CreateWidget` "/Game/HUD_messages/Normal_HUD.Normal_HUD_C" _returnvalue))
      (`UserWidget.AddToViewport` _returnvalue_2 0))
    (:`then_1`
      (bind _returnvalue_3 (`|CreateWidget` "/Game/HUD_messages/Cursor.Cursor_C"))
      (`PlayerController.SetMouseCursorWidget` _returnvalue "Default" _returnvalue_3)
      (set `PlayerController.bShowMouseCursor` true _returnvalue))
    (:`then_2`
      (`AudioComponent.Play` (`self.Audio`) 0.0))))

(event `/Game/Interactions/Enemy_Interact.Register_enemy_interact`
  ;[1 1 1] Show Death Screen
  (bind _returnvalue (`|CreateWidget` "/Game/HUD_messages/Death_Screen.Death_Screen_C" (`GameplayStatics.GetPlayerController` 0)))
  (`UserWidget.AddToViewport` _returnvalue 0))

(event `/Game/Interactions/Finish_Interact.CollectAll`
  ;[1 1 1] Win
  (`GameplayStatics.PlaySound2D` "/Game/Audio/wrd_004_Cue.wrd_004_Cue" 1.0 1.0 0.0 null null)
  (`AudioComponent.Stop` (`self.Audio`))
  (bind _returnvalue (`|CreateWidget` "/Game/HUD_messages/Win_Screen.Win_Screen_C" (`GameplayStatics.GetPlayerController` 0) :!label _label))
  (`UserWidget.AddToViewport` _returnvalue 0))

(event `/Game/Interactions/Finish_Interact.ExitLevel`
  ;[1 1 1] Win
  (goto _label))

(fn `UserConstructionScript`)