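; Reset_Wall is a one-way barrier that appears once the player passes it and resets after a teleport.
; The Cube starts invisible, and a Box overlap makes it visible with query and physics collision, without filtering which actor triggered it.
; RegisterReset hides the Cube again and disables its collision.
; Separately, RegisterLightState shows or hides a PaperSprite hidden symbol to match the incoming light state.
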(event `/Game/Interactions/ResetPoint_Interact.Register_Reset`
  (params (Reset_Point :type "/Game/Blueprints/Reset_Point Object Reference"))
  (bind _cube (`self.Cube`))
  ;[1 1 1] Reset after teleport
  (`SceneComponent.SetVisibility` _cube false true)
  (`PrimitiveComponent.SetCollisionEnabled` _cube "NoCollision"))

(event `self.ReceiveBeginPlay`
  ;[1 1 1] Start as invis
  (`SceneComponent.SetVisibility` (`self.Cube`) false true))

(event `self.Box.OnComponentBeginOverlap`
  (params (OverlappedComponent :type "PrimitiveComponent Object Reference") (OtherActor :type "Actor Object Reference") (OtherComp :type "PrimitiveComponent Object Reference") (OtherBodyIndex :type Integer) (bFromSweep :type Boolean) (SweepResult :type "HitResult Structure (by ref)"))
  (bind _cube (`self.Cube`))
  ;[1 1 1] Set visible and collision after player has passed it
  (`SceneComponent.SetVisibility` _cube true false)
  (`PrimitiveComponent.SetCollisionEnabled` _cube "QueryAndPhysics"))

(event `/Game/Interactions/Light_Interact.Register_Light_State`
  (params (Light_State :type Boolean))
  ;[1 1 1] Set visibility of hidden symbol
  (`SceneComponent.SetVisibility` (`self.PaperSprite`) Light_State false))

(fn `UserConstructionScript`)