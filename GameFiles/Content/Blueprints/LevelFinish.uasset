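; LevelFinish is a level exit trigger that checks whether the player has collected enough friends to finish.
; Any overlap with its Box runs CalcMin, which compares the TopDownCharacter's CollectedFriends against half of MaxFriends, incrementing that threshold when it falls below one.
; The resulting Check flag selects whether HUD_BLueprint shows the exit level message or the more friends needed message.
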(event `self.Box.OnComponentBeginOverlap`
  (params (OverlappedComponent :type "PrimitiveComponent Object Reference") (OtherActor :type "Actor Object Reference") (OtherComp :type "PrimitiveComponent Object Reference") (OtherBodyIndex :type Integer) (bFromSweep :type Boolean) (SweepResult :type "HitResult Structure (by ref)"))
  (`self.CalcMin`)
  (if (`self.Check`)
    (bind _ashud_blueprint (cast `/Game/Blueprints/HUD_BLueprint` (`PlayerController.GetHUD` (`GameplayStatics.GetPlayerController` 0))))
    (message `/Game/Interactions/Finish_Interact.ExitLevel` _ashud_blueprint)
    (else
      (bind _ashud_blueprint_2 (cast `/Game/Blueprints/HUD_BLueprint` (`PlayerController.GetHUD` (`GameplayStatics.GetPlayerController` 0))))
      (message `/Game/Interactions/Gate_Interact.MoreFriendsNeeded` _ashud_blueprint_2))))

(fn `CalcMin`
  (bind _collectfriend (`self.CollectFriend`))
  (bind _astop_down_character (cast `/Game/TopDownBP/Blueprints/TopDownCharacter` (`GameplayStatics.GetPlayerCharacter` 0)))
  (set `self.CollectFriend` (`/Game/TopDownBP/Blueprints/TopDownCharacter.Collected_Friends` _astop_down_character))
  (bind _returnvalue (/ (`/Game/TopDownBP/Blueprints/TopDownCharacter.MaxFriends` _astop_down_character) 2))
  (if (< _returnvalue 1)
    (bind _result (`/Engine/EditorBlueprintResources/StandardMacros.IncrementInt` _returnvalue)
      (:`  `
        (set `self.Check` (<= _result _collectfriend))))
    (else
      (set `self.Check` (<= _returnvalue _collectfriend)))))

(fn `UserConstructionScript`)