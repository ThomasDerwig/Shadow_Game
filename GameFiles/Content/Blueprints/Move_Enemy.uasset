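; Enemy character for a top-down game that moves faster than the player and gives chase, or dies to the vanquisher light.
; A player entering its sphere destroys it if VanquisherLight is active, otherwise triggers AIMoveTo without pathfinding, targeting the player controller, with an angry-cat sound on success.
; Any sphere overlap reveals its Paper sprite, whose visibility RegisterLightState also sets.
; Player overlap with its box triggers the HUD's enemy interaction message.
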(event `self.ReceiveBeginPlay`
  ;[1 1 1] Set enemy speed to be faster than player
  (set `CharacterMovementComponent.MaxWalkSpeed` 800.0 (`self.CharacterMovement`)))

(event `self.Box.OnComponentBeginOverlap`
  (params (OverlappedComponent :type "PrimitiveComponent Object Reference") (OtherActor :type "Actor Object Reference") (OtherComp :type "PrimitiveComponent Object Reference") (OtherBodyIndex :type Integer) (bFromSweep :type Boolean) (SweepResult :type "HitResult Structure (by ref)"))
  ;[1 1 1] Notify HUD of overlap
  (cast `/Game/TopDownBP/Blueprints/TopDownCharacter` OtherActor)
  (`KismetSystemLibrary.PrintString` (`KismetStringLibrary.Conv_ObjectToString` OtherActor))
  (bind _ashud_blueprint (cast `/Game/Blueprints/HUD_BLueprint` (`PlayerController.GetHUD` (`GameplayStatics.GetPlayerController` 0))))
  (message `/Game/Interactions/Enemy_Interact.Register_enemy_interact` _ashud_blueprint))

(event `self.Sphere.OnComponentBeginOverlap`
  (params (OverlappedComponent :type "PrimitiveComponent Object Reference") (OtherActor :type "Actor Object Reference") (OtherComp :type "PrimitiveComponent Object Reference") (OtherBodyIndex :type Integer) (bFromSweep :type Boolean) (SweepResult :type "HitResult Structure (by ref)"))
  ;[1 1 1] Vanquisher death OR Chase player
  (`|ExecutionSequence`
    (:`then_0`
      (bind _astop_down_character (cast `/Game/TopDownBP/Blueprints/TopDownCharacter` OtherActor))
      (`KismetSystemLibrary.PrintString` (`KismetSystemLibrary.GetDisplayName` OtherActor))
      (if (`/Game/TopDownBP/Blueprints/TopDownCharacter.Vanquisher_Light` _astop_down_character)
        (`self.K2_DestroyActor` self)
        (else
          (`AITask_MoveTo.AIMoveTo` (`AIBlueprintHelperLibrary.GetAIController` self) (1.0 1.0 1.0) (`GameplayStatics.GetPlayerController` 0) -1.0 "Default" "Default" false
            (:`then`
              (`GameplayStatics.PlaySound2D` "/Game/Audio/ANGRY_CAT_SOUND_EFFECT.ANGRY_CAT_SOUND_EFFECT" 1.0 1.0 0.0 null null))
            (:`OnRequestFailed`
              (`KismetSystemLibrary.PrintString` "Request Fail"))))))
    (:`then_1`
      (`SceneComponent.SetVisibility` (`self.PaperSprite`) true false))))

(event `/Game/Interactions/Light_Interact.Register_Light_State`
  (params (Light_State :type Boolean))
  (`SceneComponent.SetVisibility` (`self.PaperSprite`) Light_State false))

(fn `UserConstructionScript`)