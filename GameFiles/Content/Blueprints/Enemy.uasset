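; Enemy Blueprint that reacts to the player through two trigger volumes.
; Overlapping its Trigger registers the enemy's interact message with the player's HUD Blueprint.
; Overlapping the Vanquisher trigger destroys the enemy if the overlapping TopDownCharacter has VanquisherLight active.
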(event `self.trigger.OnComponentBeginOverlap`
  (params (OverlappedComponent :type "PrimitiveComponent Object Reference") (OtherActor :type "Actor Object Reference") (OtherComp :type "PrimitiveComponent Object Reference") (OtherBodyIndex :type Integer) (bFromSweep :type Boolean) (SweepResult :type "HitResult Structure (by ref)"))
  ;[1 1 1] Notify Hud of overlap
  (bind _ashud_blueprint (cast `/Game/Blueprints/HUD_BLueprint` (`PlayerController.GetHUD` (`GameplayStatics.GetPlayerController` 0))))
  (message `/Game/Interactions/Enemy_Interact.Register_enemy_interact` _ashud_blueprint self))

(event `self.Vanquisher_Trigger.OnComponentBeginOverlap`
  (params (OverlappedComponent :type "PrimitiveComponent Object Reference") (OtherActor :type "Actor Object Reference") (OtherComp :type "PrimitiveComponent Object Reference") (OtherBodyIndex :type Integer) (bFromSweep :type Boolean) (SweepResult :type "HitResult Structure (by ref)"))
  ;[1 1 1] Vanquisher light death
  (bind _astop_down_character (cast `/Game/TopDownBP/Blueprints/TopDownCharacter` OtherActor))
  (if (`/Game/TopDownBP/Blueprints/TopDownCharacter.Vanquisher_Light` _astop_down_character)
    (`self.K2_DestroyActor` self)))

(fn `UserConstructionScript`)