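; Closing wall Blueprint that starts invisible and seals permanently behind the player once they pass through its trigger.
; On the first end overlap of the trigger, it plays a thud, shows the wall in oak, enables collision and sets a Closed flag.
; Until then, RegisterLightState toggles the wall's visibility with the light state using a dark wood material, revealing it as a hidden symbol.
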(event `self.ReceiveBeginPlay`
  ;[1 1 1] Start as invis
  (`SceneComponent.SetVisibility` (`self.Closing_Wall`) false true))

(event `self.trigger.OnComponentEndOverlap`
  (params (OverlappedComponent :type "PrimitiveComponent Object Reference") (OtherActor :type "Actor Object Reference") (OtherComp :type "PrimitiveComponent Object Reference") (OtherBodyIndex :type Integer))
  (bind _closing_wall (`self.Closing_Wall`))
  ;[1 1 1] Set visible and collision after player has passed it
  (if (not (`self.Closed`))
    (`GameplayStatics.PlaySound2D` "/Game/Audio/Thud_Sound_Effect.Thud_Sound_Effect" 1.0 1.0 0.0 null null)
    (`SceneComponent.SetVisibility` _closing_wall true false)
    (set `self.Closed` true)
    (`PrimitiveComponent.SetCollisionEnabled` _closing_wall "QueryAndPhysics")
    (`PrimitiveComponent.SetMaterial` _closing_wall 0 "/Game/StarterContent/Materials/M_Wood_Oak.M_Wood_Oak")))

(event `/Game/Interactions/Light_Interact.Register_Light_State`
  (params (Light_State :type Boolean))
  (bind _closing_wall (`self.Closing_Wall`))
  ;[1 1 1] Set visibility of hidden symbol
  (if (not (`self.Closed`))
    (`SceneComponent.SetVisibility` _closing_wall Light_State false)
    (`PrimitiveComponent.SetMaterial` _closing_wall 0 "/Game/StarterContent/Materials/DarkWoodTrans.DarkWoodTrans")))

(fn `UserConstructionScript`)